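; Igloo plugin manager actor that captures a panoramic view around a followed object, or the player camera, and broadcasts it over Spout.
; It spawns attached 90-degree IglooPanoCamera actors for four sides plus optional floor and ceiling, and an optional crosshair.
; Each tick it captures them and draws them side by side in sixth-width slots on one render target.
; Command-line arguments can override sender name, camera count and resolution.
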(event EventBeginPlay
  ;[1 1 1] On Application Start
  (CallFunction|GetCommandInputs)
  (Utilities|FlowControl|Sequence
    (:then_0
      (if (Variables|Default|GetUseIglooCrosshair)
        (Utilities|CreateIglooCrosshair)))
    (:then_1
      (if (Variables|Default|GetCreateOnAwake)
        (Utilities|CreateIglooCameras)))))

(event EventTick
  (params (DeltaSeconds :type Float%20%28single-precision%29))
  ;[1 1 1] On Application Tick
  (CallFunction|UpdateFollow)
  (CallFunction|UpdateCameras))

(event EventEndPlay
  (params (EndPlayReason :type EEndPlayReason%20Enum :default "Destroyed"))
  ;[1 1 1] On Application Close / Destroyed
  (CallFunction|Cleanup))

(event EventDestroyed
  ;[1 1 1] On Application Close / Destroyed
  (CallFunction|Cleanup))

(fn ConstructionScript)

(fn GetCommandInputs
  ;[1 1 1] Checks through command lines to see if they have been provided, and adjusts the variables to suit the values given.
  (for (_array_element _array_index) (LocalVariables|GetCommandLineSearches)
    (bind _returnvalue (Utilities|GetCommandLine))
    (for _array_element_2 (Utilities|String|ParseIntoArray _returnvalue " ")
      (if (Utilities|String|Contains _array_element_2 _array_element)
        (switch int _array_index
          (:0
            ;[1 1 1] -iglooSenderName
            (Variables|Default|SetSpoutOutputName (Utilities|String|StringToName (.RightS (Utilities|String|Split _array_element_2 "=")))))
          (:1
            ;[1 1 1] -iglooNumCams
            (Variables|Default|SetNumberOfCameras (Math|Conversions|ToInteger(Byte) (.RightS (Utilities|String|Split _array_element_2 "=")))))
          (:2
            ;[1 1 1] -iglooSetResolution
            (Variables|Default|SetOutputSize (Utilities|Struct|MakeIntPoint (* (Math|Conversions|ToInteger(Byte) (.RightS (Utilities|String|Split _array_element_2 "="))) 6) (Math|Conversions|ToInteger(Byte) (.RightS (Utilities|String|Split _array_element_2 "=")))))))))))

(fn Cleanup
  (bind _igloocrosshairactor (Variables|Default|GetIglooCrosshairActor))
  (Utilities|IsValid _igloocrosshairactor
    (:Is%20Valid
      (Actor|DestroyActor _igloocrosshairactor))))

(fn DrawCamerastoCanvas
  (params (Width :type Integer) (Height :type Integer) (Canvas :type Canvas%20Object%20Reference))
  (bind _returnvalue (/ Width 6))
  (for (_array_element _array_index) (Variables|Default|GetCameraActors)
    (Default|DrawCamera _array_element Canvas (Math|Vector2D|MakeVector2D (Math|Conversions|ToFloat(Integer) (* _array_index _returnvalue)) 0.0) (Math|Vector2D|MakeVector2D (Math|Conversions|ToFloat(Integer) _returnvalue) (Math|Conversions|ToFloat(Integer) Height)))))

(fn UpdateFollow
  (bind _follow_object (Variables|Default|GetFollow%20Object))
  (Utilities|IsValid _follow_object
    (:Is%20Valid
      ;[1 1 1] Follow Object
      (Transformation|SetActorLocation (Transformation|GetActorLocation _follow_object) false true))
    (:Is%20Not%20Valid
      ;[1 1 1] Follow Player Camera
      (Transformation|SetActorLocation (Camera|GetCameraLocation (Game|GetPlayerCameraManager 0)) false true))))

(fn UpdateCameras
  (bind _equirectangularrendertarget (Variables|Default|GetEquirectangularRenderTarget))
  (bind (_width _height) (Class|CanvasRenderTarget2D|GetSize _equirectangularrendertarget))
  (for _array_element (Variables|Default|GetCameraActors)
    (Default|CaptureScene _array_element))
  (Utilities|IsValid _equirectangularrendertarget
    (:Is%20Valid
      ;[1 1 1] Draw canvas to render target
      (bind (_canvas _size _context) (Rendering|BeginDrawCanvastoRenderTarget _equirectangularrendertarget))
      (CallFunction|DrawCamerastoCanvas _width _height _canvas)
      (Rendering|EndDrawCanvastoRenderTarget _context)
      (Utilities|IsValid (Variables|Default|GetEquirectangularRenderTarget)
        (:Is%20Valid
          (Utilities|BroadcastTexture))))
    (:Is%20Not%20Valid
      (Utilities|CreateRenderTexture))))