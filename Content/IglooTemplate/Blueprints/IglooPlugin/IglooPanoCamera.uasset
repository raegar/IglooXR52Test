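; Igloo panoramic camera Blueprint that renders a scene capture to a texture and draws it onto a canvas.
; Setup creates an sRGB render target and a dynamic material carrying the texture, FOV and flip parameters.
; It builds a custom off-center-capable projection matrix from horizontal and vertical FOV angles.
; Helpers expose manual or per-frame capture, capture source, exposure and render target release.
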(event Custom|Setup%20Camera
  (params (Width :type Integer) (Height :type Integer) (Gamma :type Float%20%28double-precision%29) (HFOV :type Float%20%28double-precision%29) (VFOV :type Float%20%28double-precision%29) (Flip%20Horizontal :type Boolean) (FlipVertical :type Boolean))
  (bind _camera (Variables|Default|GetCamera))
  ;[1 1 1] Setup Camera
  (CallFunction|UpdateRenderTextures Width Height Gamma Flip%20Horizontal FlipVertical)
  ;[1 1 1] FOV System
  (Variables|Default|SetHFOV HFOV)
  (bind _output_get (Variables|Default|SetVFOV VFOV))
  (Variables|/Script/Engine.SceneCaptureComponent2D|SetFOVAngle (Variables|Default|GetCamera) _output_get)
  (bind _matrix (CallFunction|CreateFOVPerspectiveMatrix (* HFOV -0.5) (* HFOV 0.5) (* VFOV -0.5) (* VFOV 0.5) 1e+01))
  (Variables|/Script/Engine.SceneCaptureComponent2D|SetCustomProjectionMatrix _camera _matrix)
  (Variables|/Script/Engine.SceneCaptureComponent2D|SetbUseCustomProjectionMatrix _camera true))

(event Custom|Draw%20Camera
  (params (canvas :type Canvas%20Object%20Reference) (ScreenPosition :type Vector%202D%20Structure) (ScreenSize :type Vector%202D%20Structure))
  ;[1 1 1] Draw Camera
  (Canvas|DrawMaterial :self canvas :RenderMaterial (Variables|Default|GetDrawMaterialOutput) :ScreenPosition ScreenPosition :ScreenSize ScreenSize :CoordinateSize "(X=1.000000,Y=1.000000)" :PivotPoint "(X=0.500000,Y=0.500000)"))

(event Custom|Update%20Render%20Textures
  (params (Width :type Integer) (Height :type Integer) (Gamma :type Float%20%28double-precision%29) (FlipX :type Boolean) (FlipY :type Boolean))
  ;[1 1 1] Create render texture
  (Utilities|FlowControl|Sequence
    (:then_0
      (CallFunction|ClearRenderTextures)
      (bind _returnvalue (Rendering|CreateRenderTarget2D Width Height "RTF_RGBA8_SRGB"))
      (Utilities|IsValid _returnvalue
        (:Is%20Valid
          (Variables|/Script/Engine.TextureRenderTarget|SetTargetGamma _returnvalue Gamma)
          (Variables|/Script/Engine.TextureRenderTarget2D|SetAddressX _returnvalue "TA_Clamp")
          (Variables|/Script/Engine.TextureRenderTarget2D|SetAddressY _returnvalue "TA_Clamp")
          (Variables|/Script/Engine.SceneCaptureComponent2D|SetTextureTarget (Variables|Default|GetCamera) _returnvalue))))
    (:then_1
      (bind _returnvalue_2 (Rendering|Material|CreateDynamicMaterialInstance (Variables|Default|GetDrawMaterial) "None" "None" :!class /Script/Engine.KismetMaterialLibrary))
      (Rendering|Material|SetTextureParameterValue _returnvalue_2 "Texture" _returnvalue)
      (Rendering|Material|SetScalarParameterValue _returnvalue_2 "HFOV" (Variables|Default|GetHFOV) :!class /Script/Engine.MaterialInstanceDynamic)
      (Rendering|Material|SetScalarParameterValue _returnvalue_2 "VFOV" (Variables|Default|GetVFOV) :!class /Script/Engine.MaterialInstanceDynamic)
      (Rendering|Material|SetScalarParameterValue _returnvalue_2 "FlipX" (Math|Float|SelectFloat 1.0 0.0 FlipX) :!class /Script/Engine.MaterialInstanceDynamic)
      (Rendering|Material|SetScalarParameterValue _returnvalue_2 "FlipY" (Math|Float|SelectFloat 1.0 0.0 FlipY) :!class /Script/Engine.MaterialInstanceDynamic)
      (Variables|Default|SetDrawMaterialOutput _returnvalue_2))))

(event Custom|Clear%20Render%20Textures
  (bind _camera (Variables|Default|GetCamera))
  (bind _texturetarget (Variables|/Script/Engine.SceneCaptureComponent2D|GetTextureTarget _camera))
  ;[1 1 1] Clear Render Textures
  (Utilities|IsValid _texturetarget
    (:Is%20Valid
      (Class|KismetRenderingLibrary|ReleaseRenderTarget2D _texturetarget)
      (Variables|Default|SetDrawMaterialOutput 0))))

(event Custom|SetExposureCompensation
  (params (Metering%20Mode :type EAutoExposureMethod%20Enum :default "AEM_Histogram") (Exposure%20Compensation :type Float%20%28single-precision%29))
  (bind _camera (Variables|Default|GetCamera))
  ;[1 1 1] Set Exposure Compensation
  (bind _structout (Utilities|Struct|SetmembersinPostProcessSettings (Variables|/Script/Engine.SceneCaptureComponent2D|GetPostProcessSettings _camera) Metering%20Mode Exposure%20Compensation))
  (Variables|/Script/Engine.SceneCaptureComponent2D|SetPostProcessSettings _camera _structout))

(event Custom|Capture%20Scene
  ;[1 1 1] Capture Scene
  (if (not (Variables|/Script/Engine.SceneCaptureComponent|GetbCaptureEveryFrame (Variables|Default|GetCamera)))
    (Utilities|IsValid (Variables|Default|GetDrawMaterialOutput)
      (:Is%20Valid
        (Rendering|SceneCapture|CaptureScene (Variables|Default|GetCamera) :!class /Script/Engine.SceneCaptureComponent2D)))))

(event Custom|Set%20Capture%20Every%20Frame
  (params (Capture%20Every%20Frame :type Boolean))
  ;[1 1 1] Set Capture Every Frame
  (Variables|/Script/Engine.SceneCaptureComponent|SetbCaptureEveryFrame (Variables|Default|GetCamera) Capture%20Every%20Frame))

(fn ConstructionScript
  (|CallParentFunction))

(fn SetSceneCaptureSource
  (params (Capture%20Source :type ESceneCaptureSource%20Enum :default "SCS_SceneColorHDR"))
  (Variables|/Script/Engine.SceneCaptureComponent|SetCaptureSource (Variables|Default|GetCamera) Capture%20Source))

(fn CreateFOVPerspectiveMatrix
  (params (FOVLeft :type Float%20%28double-precision%29) (FOVRight :type Float%20%28double-precision%29) (FOVBottom :type Float%20%28double-precision%29) (FOVTop :type Float%20%28double-precision%29) (Near :type Float%20%28double-precision%29))
  (Utilities|FlowControl|Sequence
    (:then_0
      ;[0 0 0 1 12] Get the varaibles for the off center projection
      (LocalVariables|Setleft (Math|Trig|Tan(Degrees) FOVLeft))
      (LocalVariables|Setright (Math|Trig|Tan(Degrees) FOVRight))
      (LocalVariables|Setbottom (Math|Trig|Tan(Degrees) FOVBottom))
      (LocalVariables|Settop (Math|Trig|Tan(Degrees) FOVTop)))
    (:then_1
      ;[0 0 0 1 12] Comment
      (LocalVariables|SetsumRL (+ (LocalVariables|Getright) (LocalVariables|Getleft)))
      (LocalVariables|SetsumTB (+ (LocalVariables|Gettop) (LocalVariables|Getbottom)))
      (LocalVariables|SetinvRL (/ 1.0 (- (LocalVariables|Getright) (LocalVariables|Getleft))))
      (LocalVariables|SetinvTB (/ 1.0 (- (LocalVariables|Gettop) (LocalVariables|Getbottom))))
      (return (Utilities|Struct|MakeMatrix (Utilities|Struct|MakePlane 0.0 (* (LocalVariables|GetinvRL) 2.0) 0.0 0.0) (Utilities|Struct|MakePlane 0.0 0.0 (* (LocalVariables|GetinvTB) 2.0) 0.0) (Utilities|Struct|MakePlane 1.0 (* (LocalVariables|GetsumRL) (LocalVariables|GetinvRL)) (* (LocalVariables|GetsumTB) (LocalVariables|GetinvTB)) 0.0) (Utilities|Struct|MakePlane 0.0 0.0 0.0 Near))))))