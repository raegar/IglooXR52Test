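; World-space menu actor that hosts the WBP_UMGMain panel in a widget component and starts hidden, with collision off.
; On BeginPlay it casts the component's widget and binds to its close and quit dispatchers.
; Close hides the actor, disables collision and clears IsMenuVisible, while quit exits the game.
; Nothing in this graph shows the menu again.
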(event Custom|ClosePanel_Pressed_Event_0
  (Rendering|SetActorHiddenInGame true)
  (Collision|SetActorEnableCollision false)
  (Variables|Default|SetIsMenuVisible? false))

(event Custom|Quit%20Button_Pressed_Event
  (Game|QuitGame 0 "Quit" false))

(event EventBeginPlay
  (Rendering|SetActorHiddenInGame true)
  (Collision|SetActorEnableCollision false)
  (bind _aswbp_umgmain (Utilities|Casting|CastToWBP_UMGMain (UserInterface|GetUserWidgetObject (Variables|Default|GetWidget))))
  (bind _output_get (Variables|Default|SetAs%20WBP%20UMGMain _aswbp_umgmain))
  (EventDispatchers|AssignClosePanelPressed _output_get (delegate Custom|ClosePanel_Pressed_Event_0))
  (EventDispatchers|AssignQuitButtonPressed _output_get (delegate Custom|Quit%20Button_Pressed_Event)))

(event Collision|EventActorBeginOverlap
  (params (OtherActor :type Actor%20Object%20Reference)))

(event EventTick
  (params (DeltaSeconds :type Float%20%28single-precision%29)))

(fn ConstructionScript)